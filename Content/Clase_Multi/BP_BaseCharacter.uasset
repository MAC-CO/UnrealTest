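; BP_BaseCharacter is a base character Blueprint that tracks health, dies when it runs out, and requests a respawn.
; AnyDamage subtracts damage from Health, prints the new value, then runs a death check that destroys the actor after a brief delay at zero or below.
; On Destroyed, it casts the game mode to GM_GameModeCustom and calls RespawnCharacter with the mesh's world location.
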(event `self.ReceiveBeginPlay`
  ;[1 1 1] Print Vida on Start
  (bind _output_get (set `self.Health` (`self.Health`)))
  (`KismetSystemLibrary.PrintString` (`KismetStringLibrary.Conv_DoubleToString` _output_get) true true (struct :`R` 0.209213 :`G` 1.0 :`A` 1.0) 5.0))

(event `self.ReceiveAnyDamage`
  (params (Damage :type "Float (single-precision)") (DamageType :type "DamageType Object Reference") (InstigatedBy :type "Controller Object Reference") (DamageCauser :type "Actor Object Reference"))
  ;[1 1 1] Aplicar e imprimir daño a la vida
  (bind _output_get (set `self.Health` (- (`self.Health`) Damage)))
  (`KismetSystemLibrary.PrintString` (`KismetStringLibrary.Conv_DoubleToString` _output_get) true true (struct :`R` 1.0 :`B` 0.011367 :`A` 1.0) 5.0)
  (`self.IsDead?`))

(event `IsDead?`
  ;[1 1 1] IF vida
  (if (<= (`self.Health`) 0.0)
    (`KismetSystemLibrary.PrintString` "Muerto")
    (`KismetSystemLibrary.Delay` 0.1)
    (`self.K2_DestroyActor`)))

(event `self.ReceiveDestroyed`
  (bind _asgm_game_mode_custom (cast `/Game/Clase_Multi/GM_GameModeCustom` (`GameplayStatics.GetGameMode`)))
  (`/Game/Clase_Multi/GM_GameModeCustom.RespawnCharacter` _asgm_game_mode_custom (`SceneComponent.K2_GetComponentLocation` (`self.Mesh`))))

(fn `UserConstructionScript`)