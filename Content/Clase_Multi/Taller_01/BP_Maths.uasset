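; BP_Maths is an actor in a class workshop folder that demonstrates basic Blueprint math through debug key presses.
; Separate keys multiply two numbers, subtract three floats from a constant, or add two vectors, printing each result to screen.
; Operands come from Blueprint variables, and only the multiplication stores its result in a variable before printing.
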(event `self.ReceiveTick`
  (params (DeltaSeconds :type "Float (single-precision)")))

(event `Key|Two`
  (params (Key :type "Key Structure"))
  (:`Pressed`
    (bind _output_get (set `self.Result` (* (`self.Num1`) (`self.Num2`))))
    (`KismetSystemLibrary.PrintString` (`KismetStringLibrary.Conv_IntToString` _output_get) true true (struct :`G` 0.66 :`B` 1.0 :`A` 1.0) 5.0)))

(event `Key|Three`
  (params (Key :type "Key Structure"))
  (:`Pressed`
    (`KismetSystemLibrary.PrintString` (`KismetStringLibrary.Conv_DoubleToString` (- 100.0 (`self.Float1`) (`self.Float2`) (`self.Float3`))) true true (struct :`R` 1.0 :`B` 0.272994 :`A` 1.0))))

(event `Key|Four`
  (params (Key :type "Key Structure"))
  (:`Pressed`
    (`KismetSystemLibrary.PrintString` (`KismetStringLibrary.Conv_VectorToString` (+ (`self.Vector1`) (`self.Vector2`))))))

(fn `UserConstructionScript`)