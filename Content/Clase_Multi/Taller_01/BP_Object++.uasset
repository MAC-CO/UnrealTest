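; BP_Object++ is a coin pickup that adds one to the Coins counter of an overlapping BP_TallerCharacter and respawns afterward.
; On box overlap it disables collision, hides itself and prints the new coin total on screen.
; It then calls RespawnCoin, which uses a retriggerable delay to show the actor and restore query-only collision a few seconds later.
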(event `self.Box.OnComponentBeginOverlap`
  (params (OverlappedComponent :type "PrimitiveComponent Object Reference") (OtherActor :type "Actor Object Reference") (OtherComp :type "PrimitiveComponent Object Reference") (OtherBodyIndex :type Integer) (bFromSweep :type Boolean) (SweepResult :type "HitResult Structure (by ref)"))
  (bind _asbp_taller_character (cast `/Game/Clase_Multi/Taller_01/BP_TallerCharacter` OtherActor))
  (bind _result (`/Engine/EditorBlueprintResources/StandardMacros.IncrementInt` (`/Game/Clase_Multi/Taller_01/BP_TallerCharacter.Coins` _asbp_taller_character))
    (:`  `
      (bind _output_get (set `/Game/Clase_Multi/Taller_01/BP_TallerCharacter.Coins` _result _asbp_taller_character))
      (`PrimitiveComponent.SetCollisionEnabled` (`self.Box`) "NoCollision") ; Apago la collision
      (`self.SetActorHiddenInGame` self true) ; Ocultar el objeto
      (`KismetSystemLibrary.PrintString` (`KismetStringLibrary.Conv_IntToString` _output_get) true true (struct :`G` 1.0 :`B` 0.485975 :`A` 1.0))
      (`self.RespawnCoin`) ; Llamo el timer
    )))

(event `RespawnCoin`
  (`KismetSystemLibrary.RetriggerableDelay` 3.0)
  (`self.SetActorHiddenInGame` self false)
  (`PrimitiveComponent.SetCollisionEnabled` (`self.Box`) "QueryOnly"))

(fn `UserConstructionScript`)