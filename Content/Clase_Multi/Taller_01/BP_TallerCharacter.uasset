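; BP_TallerCharacter is a player Character from a class workshop (Taller_01) that handles basic movement, camera look, jumping and crouching through Enhanced Input.
; On BeginPlay it adds the Taller mapping context to the controlling player's Enhanced Input subsystem.
; The Run action moves along right and forward vectors derived from control rotation, and Look drives controller yaw and pitch.
; Jump and Crouch start on Triggered and end on Completed.
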(event `self.ReceiveTick`
  (params (DeltaSeconds :type "Float (single-precision)")))

(event `self.ReceiveBeginPlay`
  ;[1 1 1] Comment
  (bind _asplayer_controller (cast `PlayerController` (`self.GetController`)))
  (bind _returnvalue (pcsubsystem `EnhancedInputLocalPlayerSubsystem` _asplayer_controller))
  (`/Engine/EditorBlueprintResources/StandardMacros.IsValid` _returnvalue
    (:`Is Valid`
      (`EnhancedInputSubsystemInterface.AddMappingContext` _returnvalue "/Game/Clase_Multi/Taller_01/Taller_MappingContext.Taller_MappingContext" 0 (struct)))))

(event `EnhancedInput|/Game/Clase_Multi/Taller_01/Taller_Look`
  (params (ActionValue :type "Vector2D Structure") (ElapsedSeconds :type "Float (double-precision)") (TriggeredSeconds :type "Float (double-precision)") (InputAction :type "InputAction Object Reference" :default "/Game/Clase_Multi/Taller_01/Taller_Look.Taller_Look"))
  ;[1 1 1] Comment
  (:`Triggered`
    (`self.AddControllerYawInput` ActionValue_X)
    (`self.AddControllerPitchInput` ActionValue_Y)))

(event `EnhancedInput|/Game/Clase_Multi/Taller_01/Taller_Run`
  (params (ActionValue :type "Vector2D Structure") (ElapsedSeconds :type "Float (double-precision)") (TriggeredSeconds :type "Float (double-precision)") (InputAction :type "InputAction Object Reference" :default "/Game/Clase_Multi/Taller_01/Taller_Run.Taller_Run"))
  (bind (_returnvalue_roll _returnvalue_pitch _returnvalue_yaw) (`KismetMathLibrary.BreakRotator` (`self.GetControlRotation`)))
  (bind (_returnvalue_roll_2 _returnvalue_pitch_2 _returnvalue_yaw_2) (`KismetMathLibrary.BreakRotator` (`self.GetControlRotation`)))
  ;[1 1 1] Comment
  (:`Triggered`
    (`self.AddMovementInput` (`KismetMathLibrary.GetRightVector` (`KismetMathLibrary.MakeRotator` _returnvalue_roll_2 0.0 _returnvalue_yaw_2)) ActionValue_X)
    (`self.AddMovementInput` (`KismetMathLibrary.GetForwardVector` (`KismetMathLibrary.MakeRotator` 0.0 0.0 _returnvalue_yaw)) ActionValue_Y)))

(event `EnhancedInput|/Game/Clase_Multi/Taller_01/Taller_Jump`
  (params (ActionValue :type Boolean) (ElapsedSeconds :type "Float (double-precision)") (TriggeredSeconds :type "Float (double-precision)") (InputAction :type "InputAction Object Reference" :default "/Game/Clase_Multi/Taller_01/Taller_Jump.Taller_Jump"))
  ;[1 1 1] Comment
  (:`Triggered`
    (`self.Jump`))
  (:`Completed`
    (`self.StopJumping`)))

(event `Key|LeftControl`
  (params (Key :type "Key Structure")))

(event `EnhancedInput|/Game/Clase_Multi/Taller_01/Taller_Crounch`
  (params (ActionValue :type Boolean) (ElapsedSeconds :type "Float (double-precision)") (TriggeredSeconds :type "Float (double-precision)") (InputAction :type "InputAction Object Reference" :default "/Game/Clase_Multi/Taller_01/Taller_Crounch.Taller_Crounch"))
  (:`Triggered`
    (`self.Crouch`))
  (:`Completed`
    (`self.UnCrouch`)))

(fn `UserConstructionScript`
  (`parent.UserConstructionScript`))