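; BP_PlatformSpline is a moving platform that travels back and forth along a spline, starting at BeginPlay.
; The Movement timeline's TravelDistance track, scaled by spline length, samples the spline to set the mesh's world location and local rotation each update.
; Rotation keeps the spline's roll and yaw but zeroes pitch.
; On Finished, a FlipFlop alternates between ReversePlatform and playing from start, looping the motion.
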(event `self.ReceiveBeginPlay`
  (bind _platform_mesh (`self.Platform Mesh`))
  (bind _spline (`self.Spline`))
  (bind (_returnvalue_roll _returnvalue_pitch _returnvalue_yaw) (`KismetMathLibrary.BreakRotator` (`SplineComponent.GetRotationAtDistanceAlongSpline` (`self.Spline`) 0.0 "Local")))
  ;[1 1 1] Comment
  (`SceneComponent.K2_SetRelativeRotation` (`self.Platform Mesh`) (`KismetMathLibrary.MakeRotator` _returnvalue_roll 0.0 _returnvalue_yaw) false false)
  ;[1 1 1] Boloñesa
  (bind (_direction _traveldistance) (`Timeline|Movement` :!label _label) ; Dar ruta a la plataforma
    (:`Update`
      (bind _returnvalue (* _traveldistance (`SplineComponent.GetSplineLength` _spline)))
      (`SceneComponent.K2_SetWorldLocation` _platform_mesh (`SplineComponent.GetLocationAtDistanceAlongSpline` _spline _returnvalue "World") false false)
      (bind (_returnvalue_roll_2 _returnvalue_pitch_2 _returnvalue_yaw_2) (`KismetMathLibrary.BreakRotator` (`SplineComponent.GetRotationAtDistanceAlongSpline` _spline _returnvalue "Local")))
      (`SceneComponent.K2_SetRelativeRotation` _platform_mesh (`KismetMathLibrary.MakeRotator` _returnvalue_roll_2 0.0 _returnvalue_yaw_2) false false))
    (:`Finished`
      (`/Engine/EditorBlueprintResources/StandardMacros.FlipFlop`
        (:`A`
          (`self.ReversePlatform`))
        (:`B`
          (goto _label :!via `PlayFromStart`))))))

(event `ReversePlatform`
  (goto _label :!via `Reverse`))

(fn `UserConstructionScript`)