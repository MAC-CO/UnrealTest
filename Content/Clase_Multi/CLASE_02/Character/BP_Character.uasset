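; BP_Character is a player-controlled Character with basic look, move and jump controls using Enhanced Input.
; On BeginPlay it casts its controller to PlayerController and adds the IMC_PlayerInputs mapping context to that player's input subsystem.
; IALook drives controller yaw and pitch, while IAMov moves along control-rotation forward and right vectors with pitch zeroed.
; IAJump starts the jump on Triggered and stops it on Completed.
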(event `self.ReceiveBeginPlay`
  ;[1 1 1] Comment
  (bind _asplayer_controller (cast `PlayerController` (`self.GetController`))) ; Referencia Controlador del Player
  (bind _returnvalue (pcsubsystem `EnhancedInputLocalPlayerSubsystem` _asplayer_controller))
  (`/Engine/EditorBlueprintResources/StandardMacros.IsValid` _returnvalue
    (:`Is Valid`
      (`EnhancedInputSubsystemInterface.AddMappingContext` _returnvalue "/Game/Clase_Multi/CLASE_02/Character/CharacterInput/IMC_PlayerInputs.IMC_PlayerInputs" 1 (struct)))))

(event `EnhancedInput|/Game/Clase_Multi/CLASE_02/Character/CharacterInput/IALook`
  (params (ActionValue :type "Vector2D Structure") (ElapsedSeconds :type "Float (double-precision)") (TriggeredSeconds :type "Float (double-precision)") (InputAction :type "InputAction Object Reference" :default "/Game/Clase_Multi/CLASE_02/Character/CharacterInput/IALook.IALook"))
  ;[1 1 1] Comment
  (:`Triggered`
    (`self.AddControllerYawInput` ActionValue_X)
    (`self.AddControllerPitchInput` ActionValue_Y)))

(event `EnhancedInput|/Game/Clase_Multi/CLASE_02/Character/CharacterInput/IAMov`
  (params (ActionValue :type "Vector2D Structure") (ElapsedSeconds :type "Float (double-precision)") (TriggeredSeconds :type "Float (double-precision)") (InputAction :type "InputAction Object Reference" :default "/Game/Clase_Multi/CLASE_02/Character/CharacterInput/IAMov.IAMov"))
  (bind (_returnvalue_roll _returnvalue_pitch _returnvalue_yaw) (`KismetMathLibrary.BreakRotator` (`self.GetControlRotation`)))
  (bind (_returnvalue_roll_2 _returnvalue_pitch_2 _returnvalue_yaw_2) (`KismetMathLibrary.BreakRotator` (`self.GetControlRotation`)))
  ;[1 1 1] Comment
  (:`Triggered`
    (`self.AddMovementInput` (`KismetMathLibrary.GetRightVector` (`KismetMathLibrary.MakeRotator` _returnvalue_roll_2 0.0 _returnvalue_yaw_2)) ActionValue_X)
    (`self.AddMovementInput` (`KismetMathLibrary.GetForwardVector` (`KismetMathLibrary.MakeRotator` 0.0 0.0 _returnvalue_yaw)) ActionValue_Y)))

(event `EnhancedInput|/Game/Clase_Multi/CLASE_02/Character/CharacterInput/IAJump`
  (params (ActionValue :type Boolean) (ElapsedSeconds :type "Float (double-precision)") (TriggeredSeconds :type "Float (double-precision)") (InputAction :type "InputAction Object Reference" :default "/Game/Clase_Multi/CLASE_02/Character/CharacterInput/IAJump.IAJump"))
  ;[1 1 1] Comment
  (:`Triggered`
    (`self.Jump`))
  (:`Completed`
    (`self.StopJumping`)))

(fn `UserConstructionScript`)